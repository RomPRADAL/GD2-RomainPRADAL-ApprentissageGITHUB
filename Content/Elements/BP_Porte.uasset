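; Door actor that moves its static mesh through two separate mechanisms, a swing and a positional toggle.
; OpenDoor and CloseDoor set the Open flag and play timelines that rotate the mesh yaw from zero in opposite directions, so closing does not reverse the opening swing.
; Activate and Desactivate both call ChangeState, which snaps the mesh between origin and a Y offset based on its current location, printing a debug message.
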(event `OpenDoor`
  (set `self.Open` true)
  (bind (_direction _newtrack_0) (`Timeline|Timeline` :!via `PlayFromStart`)
    (:`Update`
      (`SceneComponent.K2_SetRelativeRotation` (`self.StaticMesh`) (`KismetMathLibrary.MakeRotator` 0.0 0.0 (`KismetMathLibrary.Lerp` 0.0 90.0 _newtrack_0)) false false))))

(event `CloseDoor`
  (set `self.Open` false)
  (bind (_direction _newtrack_0) (`Timeline|Timeline_0` :!via `PlayFromStart`)
    (:`Update`
      (`SceneComponent.K2_SetRelativeRotation` (`self.StaticMesh`) (`KismetMathLibrary.MakeRotator` 0.0 0.0 (`KismetMathLibrary.Lerp` 0.0 -90.0 _newtrack_0)) false false))))

(event `/Game/Elements/BPI_InterrupteurControllable.Desactivate`
  (`self.ChangeState`))

(event `/Game/Elements/BPI_InterrupteurControllable.Activate`
  (`self.ChangeState`))

(fn `ChangeState`
  (bind (_relativelocation_x _relativelocation_y) (`KismetMathLibrary.BreakVector` (`SceneComponent.RelativeLocation` (`self.StaticMesh`))))
  (if (>= _relativelocation_y 10.0)
    (`KismetSystemLibrary.PrintString` "Je me ferme")
    (`SceneComponent.K2_SetRelativeLocation` (`self.StaticMesh`) (0.0 0.0 0.0) false false)
    (else
      (`KismetSystemLibrary.PrintString` "Je m'ouvre")
      (`SceneComponent.K2_SetRelativeLocation` (`self.StaticMesh`) (0.0 100.0 0.0) false false))))

(fn `UserConstructionScript`)