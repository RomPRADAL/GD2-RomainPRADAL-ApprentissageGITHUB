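; BP_PorteDrivenByEvent is a door that toggles open or closed when an external event launcher fires.
; On BeginPlay it binds its Activation event to the ActivatesControlables dispatcher on its EventLauncher reference.
; Each activation calls ChangeState, which infers the current state from the mesh's relative Y position rather than a stored flag.
; The mesh snaps between closed and offset positions without interpolation or sweep, printing a French debug message each time.
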(event `self.ReceiveBeginPlay`
  (add `/Game/Elements/BP_InterrupteurGeneralDrivenByEvent.ActivatesControlables` (`self.EventLauncher`) (delegate `Activation`)))

(event `Activation`
  (`self.ChangeState`))

(fn `ChangeState`
  (bind (_relativelocation_x _relativelocation_y) (`KismetMathLibrary.BreakVector` (`SceneComponent.RelativeLocation` (`self.StaticMesh`))))
  (if (>= _relativelocation_y 10.0)
    (`KismetSystemLibrary.PrintString` "Je me ferme")
    (`SceneComponent.K2_SetRelativeLocation` (`self.StaticMesh`) (0.0 0.0 0.0) false false)
    (else
      (`KismetSystemLibrary.PrintString` "Je m'ouvre")
      (`SceneComponent.K2_SetRelativeLocation` (`self.StaticMesh`) (0.0 100.0 0.0) false false))))

(fn `UserConstructionScript`)